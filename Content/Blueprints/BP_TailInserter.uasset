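; BP_TailInserter is a helper actor that creates the first tail segment of a grid-based snake.
; InitTail spawns a BP_TailItem one cell behind the given head position along negative X and stores that spot as LastItemPos.
; It gives the new segment the head's current direction and a reference to SnakeHead, then returns it.
; The offset always uses X regardless of heading, and the event graph is empty.
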(event EventBeginPlay)

(event Collision|EventActorBeginOverlap
  (params (OtherActor :type Actor%20Object%20Reference)))

(event EventTick
  (params (DeltaSeconds :type Float%20%28single-precision%29)))

(fn ConstructionScript)

(fn InitTail
  (params (HeadPosition :type Vector))
  (bind (_x _y _z) (Math|Vector|BreakVector HeadPosition))
  (bind _snakehead (Variables|Default|GetSnakeHead))
  (bind _cellsize (Variables|/Game/Blueprints/BP_Player.BP_Player_C|GetCellSize _snakehead))
  (bind _returnvalue (- _x _cellsize))
  (bind _returnvalue_2 (Math|Vector|MakeVector _returnvalue _y _z))
  (Variables|Default|SetLastItemPos _returnvalue_2)
  (bind _returnvalue_3 (Game|SpawnActorfromClass "/Game/Blueprints/BP_TailItem.BP_TailItem_C" (Math|Transform|MakeTransform _returnvalue_2 "0, 0, 0" "1,1,1") "Undefined" 0 0))
  (Variables|/Game/Blueprints/BP_TailItem.BP_TailItem_C|SetCurrentDirection _returnvalue_3 (Variables|/Game/Blueprints/BP_Player.BP_Player_C|GetCurrentSnakeDirection _snakehead))
  (Variables|/Game/Blueprints/BP_TailItem.BP_TailItem_C|SetHead _returnvalue_3 (Variables|Default|GetSnakeHead))
  (return _returnvalue_3))