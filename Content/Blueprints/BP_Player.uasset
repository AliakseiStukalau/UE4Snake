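; Player-controlled head of a grid-based Snake game, moving continuously each tick while the game is on; holding PauseSnake halts it.
; Turn inputs reject same-axis changes and store a desired direction, applied only when the head's bounds come close to a cell boundary.
; On BeginPlay it places itself on the grid and has the level's BP_TailInserter create the tail, then passes position and direction to the next segment every tick.
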(event EventBeginPlay
  (CallFunction|SetupSnakeHead)
  (Variables|Default|Set TresholdInaccuracyValue (* (Variables|Default|GetCellSize) 1.0))
  (bind _outactors (Actor|GetAllActorsOfClass "/Game/Blueprints/BP_TailInserter.BP_TailInserter_C"))
  (Utilities|IsValid (Utilities|Array|Get(acopy) _outactors)
    (:Is%20Valid
      (bind _output_get (Variables|Default|SetTailInserter (Utilities|Array|Get(acopy) _outactors)))
      (Variables|/Game/Blueprints/BP_TailInserter.BP_TailInserter_C|SetSnakeHead _output_get self)
      (bind _inittailitem (Default|InitTail _output_get (Transformation|GetActorLocation)))
      (Variables|Default|SetNextItem _inittailitem))
    (:Is%20Not%20Valid
      (Development|PrintString "Tail no valid" true true "(R=1.000000,G=0.023580,B=0.000000,A=1.000000)" 2e+01))))

(event Collision|EventActorBeginOverlap
  (params (OtherActor :type Actor%20Object%20Reference)))

(event EventTick
  (params (DeltaSeconds :type Float%20%28single-precision%29))
  (if (Variables|Default|GetIsGameOn)
    (bind (_offset _currentdirection) (CallFunction|CalculateOffsetandDirection DeltaSeconds))
    (Transformation|AddActorLocalOffset _offset true true)
    (Default|UpdatePosition (Variables|Default|GetNextItem) (Transformation|GetActorLocation) _currentdirection)))

(event Input|ActionEvents|InputActionTurnRight
  (params (Key :type Key%20Structure :default "None"))
  (:Pressed
    (bind _position (CallFunction|GetActorBoundStartPos))
    (bind _canturn (CallFunction|IsPossibletoTurn (.x _position) (Variables|Default|Get TresholdInaccuracyValue)))
    (if _canturn
      (if (== (.y (Variables|Default|GetCurrentSnakeDirection)) 0.0)
        (Variables|Default|SetDesiredSnakeDirection "0,1.000000, 0")))))

(event Input|ActionEvents|InputActionTurnUp
  (params (Key :type Key%20Structure :default "None"))
  (:Pressed
    (bind _position (CallFunction|GetActorBoundStartPos))
    (bind _canturn (CallFunction|IsPossibletoTurn (.y _position) (Variables|Default|Get TresholdInaccuracyValue)))
    (if _canturn
      (if (== (.x (Variables|Default|GetCurrentSnakeDirection)) 0.0)
        (Variables|Default|SetDesiredSnakeDirection "1.000000,0.000000, 0")))))

(event Input|ActionEvents|InputActionTurnDown
  (params (Key :type Key%20Structure :default "None"))
  (:Pressed
    (bind _position (CallFunction|GetActorBoundStartPos))
    (bind _canturn (CallFunction|IsPossibletoTurn (.y _position) (Variables|Default|Get TresholdInaccuracyValue)))
    (if _canturn
      (if (== (.x (Variables|Default|GetCurrentSnakeDirection)) 0.0)
        (Variables|Default|SetDesiredSnakeDirection "-1.000000,0.000000, 0")))))

(event Input|ActionEvents|InputActionTurnLeft
  (params (Key :type Key%20Structure :default "None"))
  (:Pressed
    (bind _position (CallFunction|GetActorBoundStartPos))
    (bind _canturn (CallFunction|IsPossibletoTurn (.x _position) (Variables|Default|Get TresholdInaccuracyValue)))
    (if _canturn
      (if (== (.y (Variables|Default|GetCurrentSnakeDirection)) 0.0)
        (Variables|Default|SetDesiredSnakeDirection "0,-1.000000, 0")))))

(event Input|ActionEvents|InputActionPauseSnake
  (params (Key :type Key%20Structure :default "None"))
  (:Pressed
    (Variables|Default|SetIsGameOn false))
  (:Released
    (Variables|Default|SetIsGameOn true)))

(fn ConstructionScript)

(fn GetActorBoundStartPos
  (return (- (Transformation|GetActorLocation) (.BoxExtent (Collision|GetActorBounds false false)))))

(fn IsPossibletoTurn
  (params (CurrentPosition :type Float%20%28single-precision%29) (Treshold :type Float%20%28single-precision%29))
  (bind _currentsnakedirection (Variables|Default|GetCurrentSnakeDirection))
  (bind _cellsize (Variables|Default|GetCellSize))
  (bind (_x _y) (Math|Vector|BreakVector _currentsnakedirection))
  (bind _returnvalue (Math|Float|%(Float) CurrentPosition _cellsize))
  (bind _returnvalue_2 (Math|Float|Absolute(Float) _returnvalue))
  (if (or (< _x 0.0) (< _y 0.0))
    (LocalVariables|SetDistanceLeft _returnvalue_2)
    (else
      (LocalVariables|SetDistanceLeft (- (Variables|Default|GetCellSize) _returnvalue_2))))
  (return (< (LocalVariables|GetDistanceLeft) Treshold)))

(fn SetupSnakeHead
  (bind _cellsize (Variables|Default|GetCellSize))
  (bind _returnvalue (* _cellsize 10.5))
  (Rendering|Material|CreateDynamicMaterialInstance (Variables|Default|GetSnakeHead) 0 "/Game/Materials/M_Snake.M_Snake" "None" :!class /Script/Engine.PrimitiveComponent)
  (Transformation|SetActorLocation (Math|Vector|MakeVector _returnvalue _returnvalue 3.0) false true))

(fn CalculateOffsetandDirection
  (params (DeltaSeconds :type Float%20%28single-precision%29))
  (bind _desiredsnakedirection (Variables|Default|GetDesiredSnakeDirection))
  (LocalVariables|SetCurrentDirectionTemp (Variables|Default|GetCurrentSnakeDirection))
  (if (Math|Vector|Equal(Vector) (Variables|Default|GetCurrentSnakeDirection) _desiredsnakedirection 0.0001)
    _
    (else
      (bind _position (CallFunction|GetActorBoundStartPos))
      (if (== (.X (Math|Vector|BreakVector _desiredsnakedirection)) 0.0)
        ;[1 1 1] Right-Left
        (bind _canturn (CallFunction|IsPossibletoTurn (.x _position) 2.0))
        (if _canturn
          (Variables|Default|SetCurrentSnakeDirection (Variables|Default|GetDesiredSnakeDirection) :!label _label))
        (else
          ;[1 1 1] Up-Down
          (bind _canturn_2 (CallFunction|IsPossibletoTurn (.y _position) 2.0))
          (if _canturn_2
            (goto _label)
            (else
              _))))))
  (return (* (Variables|Default|GetCurrentSnakeDirection) (* DeltaSeconds (Variables|Default|Get SnakeSpeed))) (LocalVariables|GetCurrentDirectionTemp)))