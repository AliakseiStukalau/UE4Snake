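; BP_TailItem is one segment of a tail chain that follows a Head actor, apparently for a snake-style game.
; UpdatePosition moves it along its current direction by the summed offset, taking the front item's previous direction on a turn and its current direction once distance since that turn reaches the head's cell size.
; It then recursively updates NextItem, passing its own direction as the previous one, so no Tick logic is used.
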(event EventBeginPlay)

(event Collision|EventActorBeginOverlap
  (params (OtherActor :type Actor%20Object%20Reference)))

(event EventTick
  (params (DeltaSeconds :type Float%20%28single-precision%29)))

(fn ConstructionScript)

(fn UpdatePosition
  (params (FrontItemPosition :type Vector) (PreviousCenterPosition :type Vector) (Offset :type Vector) (FrontItemPreviousDirection :type Vector) (FrontItemCurrentDirection :type Vector) (NewDirectionNow :type Boolean))
  (bind (_x _y _z) (Math|Vector|BreakVector Offset))
  (bind _nextitem (Variables|Default|GetNextItem))
  (bind _returnvalue (+ _x _y _z))
  (bind _returnvalue_2 (Math|Float|Absolute(Float) _returnvalue))
  (if NewDirectionNow
    (Variables|Default|SetCurrentDirection FrontItemPreviousDirection)
    (Variables|Default|SetDistanceWithoutTurns 0.0))
  (bind _output_get (Variables|Default|SetDistanceWithoutTurns (+ (Variables|Default|GetDistanceWithoutTurns) _returnvalue_2)))
  (if (<= (Variables|/Game/Blueprints/BP_Player.BP_Player_C|GetCellSize (Variables|Default|GetHead)) _output_get)
    (Variables|Default|SetCurrentDirection FrontItemCurrentDirection))
  (Transformation|AddActorLocalOffset (* (Variables|Default|GetCurrentDirection) _returnvalue_2) false false)
  (Utilities|IsValid _nextitem
    (:Is%20Valid
      (CallFunction|UpdatePosition _nextitem (Transformation|GetActorLocation) "0, 0, 0" Offset (Variables|Default|GetCurrentDirection) "0, 0, 0" NewDirectionNow))))